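; Trigger volume for ladders and walls that links their climb settings to the climbing component of a side-scroller or Paper2D character.
; The construction script sizes the box from the parent ladder or wall dimensions.
; Overlap caches the character and passes climb-through, plus horizontal for the side-scroller only.
; Events toggle the parent's attached flag and detach the character, while Tick feeds the parent's top height to the climber when attached.
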(event OnComponentBeginOverlap(Box)
  (params (OverlappedComponent :type Primitive%20Component%20Object%20Reference) (OtherActor :type Actor%20Object%20Reference) (OtherComp :type Primitive%20Component%20Object%20Reference) (OtherBodyIndex :type Integer) (bFromSweep :type Boolean) (SweepResult :type Hit%20Result%20Structure%20%28by%20ref%29))
  ;[0.2611 1 0.7352 1 30] Comment
  (Utilities|FlowControl|Sequence
    (:then_0
      ;;[1 0 0 1 30] Replace with own character
      (bind _asside_scroller_character (Utilities|Casting|CastToSideScrollerCharacter OtherActor))
      (bind _output_get (Variables|Default|SetCharacter _asside_scroller_character))
      (Variables|Default|SetOverlap true)
      (Variables|/Game/2DLadders/BluePrints/Components/BP_Climbing.BP_Climbing_C|SetClimbThrough (Variables|/Game/SideScrollerBP/Blueprints/SideScrollerCharacter.SideScrollerCharacter_C|GetBP_Climbing _output_get) (Variables|Default|GetClimbThrough))
      (Variables|/Game/2DLadders/BluePrints/Components/BP_Climbing.BP_Climbing_C|SetHorizontal (Variables|/Game/SideScrollerBP/Blueprints/SideScrollerCharacter.SideScrollerCharacter_C|GetBP_Climbing _output_get) (Variables|Default|GetHorizontal)))
    (:then_1
      (bind _asbp_paper_ladder_character (Utilities|Casting|CastToBP_PaperLadderCharacter OtherActor))
      (Variables|Default|Set2DCharacter _asbp_paper_ladder_character)
      (Variables|Default|SetOverlap true)
      (Variables|/Game/2DLadders/BluePrints/Components/BP_ClimbingPaper2D.BP_ClimbingPaper2D_C|SetClimbThrough (Variables|/Game/2DLadders/BluePrints/Characters/BP_PaperLadderCharacter.BP_PaperLadderCharacter_C|GetBP_ClimbingPaper2D _asbp_paper_ladder_character) (Variables|Default|GetClimbThrough)))))

(event OnComponentEndOverlap(Box)
  (params (OverlappedComponent :type Primitive%20Component%20Object%20Reference) (OtherActor :type Actor%20Object%20Reference) (OtherComp :type Primitive%20Component%20Object%20Reference) (OtherBodyIndex :type Integer))
  ;[0.2611 1 0.7352 1 30] Comment
  ;;[1 0 0 1 30] Replace with own character
  (Utilities|Casting|CastToSideScrollerCharacter OtherActor)
  (Variables|Default|SetOverlap false))

(event Custom|DetachFromLadder
  (bind _ladderparent (Variables|Default|GetLadderParent))
  (bind _2dcharacter (Variables|Default|Get2DCharacter))
  (bind _character (Variables|Default|GetCharacter))
  (bind _ladderparent_2 (Variables|Default|GetLadderParent))
  ;[1 0.98 0.1818 1 30] Comment
  (Utilities|IsValid _character
    (:Is%20Valid
      (Utilities|IsValid _ladderparent
        (:Is%20Valid
          (Variables|/Game/2DLadders/BluePrints/Climbables/BP_Ladder.BP_Ladder_C|SetAttached _ladderparent false)
          (Transformation|DetachFromActor _character "KeepWorld" "KeepWorld" "KeepWorld"))))
    (:Is%20Not%20Valid
      (Utilities|IsValid _2dcharacter
        (:Is%20Valid
          (Utilities|IsValid _ladderparent_2
            (:Is%20Valid
              (Variables|/Game/2DLadders/BluePrints/Climbables/BP_Ladder.BP_Ladder_C|SetAttached _ladderparent_2 false)
              (Transformation|DetachFromActor _2dcharacter "KeepWorld" "KeepWorld" "KeepWorld"))))))))

(event Custom|AttachedToLadder
  (bind _ladderparent (Variables|Default|GetLadderParent))
  ;[0.3062 0.5219 1 1 30] Comment
  (Utilities|IsValid _ladderparent
    (:Is%20Valid
      (Variables|/Game/2DLadders/BluePrints/Climbables/BP_Ladder.BP_Ladder_C|SetAttached _ladderparent true))))

(event Custom|AttachedToWall
  (bind _wallparent (Variables|Default|GetWallParent))
  ;[0.3062 0.5219 1 1 30] Comment
  (Utilities|IsValid _wallparent
    (:Is%20Valid
      (Variables|/Game/2DLadders/BluePrints/Climbables/BP_ClimbWall.BP_ClimbWall_C|SetAttached _wallparent true))))

(event Custom|DetachFromWall
  (bind _wallparent (Variables|Default|GetWallParent))
  (bind _2dcharacter (Variables|Default|Get2DCharacter))
  (bind _wallparent_2 (Variables|Default|GetWallParent))
  (bind _character (Variables|Default|GetCharacter))
  ;[1 0.98 0.1818 1 30] Comment
  (Utilities|IsValid _character
    (:Is%20Valid
      (Utilities|IsValid _wallparent_2
        (:Is%20Valid
          (Variables|/Game/2DLadders/BluePrints/Climbables/BP_ClimbWall.BP_ClimbWall_C|SetAttached _wallparent_2 false)
          (Transformation|DetachFromActor _character "KeepWorld" "KeepWorld" "KeepWorld"))))
    (:Is%20Not%20Valid
      (Utilities|IsValid _2dcharacter
        (:Is%20Valid
          (Utilities|IsValid _wallparent
            (:Is%20Valid
              (Variables|/Game/2DLadders/BluePrints/Climbables/BP_ClimbWall.BP_ClimbWall_C|SetAttached _wallparent false)
              (Transformation|DetachFromActor _2dcharacter "KeepWorld" "KeepWorld" "KeepWorld"))))))))

(event EventBeginPlay
  (bind _ladderparent (Variables|Default|GetLadderParent))
  ;[1 0.3915 0.3417 1 30] Comment
  (Utilities|IsValid _ladderparent
    (:Is%20Valid
      (Variables|Default|SetClimbThrough (Variables|/Game/2DLadders/BluePrints/Climbables/BP_Ladder.BP_Ladder_C|GetClimbThrough _ladderparent)))))

(event EventTick
  (params (DeltaSeconds :type Float%20%28single-precision%29))
  (bind _wallparent (Variables|Default|GetWallParent))
  (bind _2dcharacter (Variables|Default|Get2DCharacter))
  (bind _character (Variables|Default|GetCharacter))
  (bind _2dcharacter_2 (Variables|Default|Get2DCharacter))
  (bind _ladderparent (Variables|Default|GetLadderParent))
  (bind _topz (Variables|/Game/2DLadders/BluePrints/Climbables/BP_Ladder.BP_Ladder_C|GetTopZ _ladderparent))
  ;[0.2448 0.07891 0.2033 1 30] Set the top of the climb object
  (Utilities|IsValid _wallparent
    (:Is%20Valid
      (if (Variables|/Game/2DLadders/BluePrints/Climbables/BP_ClimbWall.BP_ClimbWall_C|GetAttached _wallparent)
        (Utilities|IsValid (Variables|Default|GetCharacter)
          (:Is%20Valid
            (bind _output_get (Variables|Default|SetTop (Variables|/Game/2DLadders/BluePrints/Climbables/BP_ClimbWall.BP_ClimbWall_C|GetTopZ _wallparent)))
            (Variables|/Game/2DLadders/BluePrints/Components/BP_Climbing.BP_Climbing_C|SetTop (Variables|/Game/SideScrollerBP/Blueprints/SideScrollerCharacter.SideScrollerCharacter_C|GetBP_Climbing (Variables|Default|GetCharacter)) _output_get))
          (:Is%20Not%20Valid
            (Utilities|IsValid _2dcharacter
              (:Is%20Valid
                (bind _output_get_2 (Variables|Default|SetTop (Variables|/Game/2DLadders/BluePrints/Climbables/BP_ClimbWall.BP_ClimbWall_C|GetTopZ _wallparent)))
                (Variables|/Game/2DLadders/BluePrints/Components/BP_ClimbingPaper2D.BP_ClimbingPaper2D_C|SetTop (Variables|/Game/2DLadders/BluePrints/Characters/BP_PaperLadderCharacter.BP_PaperLadderCharacter_C|GetBP_ClimbingPaper2D _2dcharacter) _output_get_2)))))))
    (:Is%20Not%20Valid
      (Utilities|IsValid _ladderparent
        (:Is%20Valid
          (if (Variables|/Game/2DLadders/BluePrints/Climbables/BP_Ladder.BP_Ladder_C|GetAttached _ladderparent)
            (Utilities|IsValid _character
              (:Is%20Valid
                (bind _output_get_3 (Variables|Default|SetTop _topz))
                (Variables|/Game/2DLadders/BluePrints/Components/BP_Climbing.BP_Climbing_C|SetTop (Variables|/Game/SideScrollerBP/Blueprints/SideScrollerCharacter.SideScrollerCharacter_C|GetBP_Climbing _character) _output_get_3))
              (:Is%20Not%20Valid
                (Utilities|IsValid _2dcharacter_2
                  (:Is%20Valid
                    (bind _output_get_4 (Variables|Default|SetTop _topz))
                    (Variables|/Game/2DLadders/BluePrints/Components/BP_ClimbingPaper2D.BP_ClimbingPaper2D_C|SetTop (Variables|/Game/2DLadders/BluePrints/Characters/BP_PaperLadderCharacter.BP_PaperLadderCharacter_C|GetBP_ClimbingPaper2D _2dcharacter_2) _output_get_4)))))))))))

(fn ConstructionScript
  (bind _ladderparent (Variables|Default|GetLadderParent))
  (bind _wallparent (Variables|Default|GetWallParent))
  (bind _ladderparent_2 (Variables|Default|GetLadderParent))
  (switch Utilities|FlowControl|Switch|SwitchonEnum_climbable (Variables|Default|GetType)
    (:NewEnumerator0
      (if (Variables|Default|GetHorizontal)
        (Variables|Default|SetTypeSub (Variables|/Game/2DLadders/BluePrints/Climbables/BP_Ladder.BP_Ladder_C|GetSubType _ladderparent_2))
        (Components|Box|SetBoxExtent (Variables|Default|GetBox) (Math|Vector|MakeVector 15.0 15.0 (* (Math|Conversions|ToFloat(Integer) (Variables|/Game/2DLadders/BluePrints/Climbables/BP_Ladder.BP_Ladder_C|GetLength _ladderparent_2)) (/ (Variables|/Game/2DLadders/BluePrints/Climbables/BP_Ladder.BP_Ladder_C|GetSectionSize _ladderparent_2) 2.3))) true)
        (else
          (Variables|Default|SetTop (Variables|/Game/2DLadders/BluePrints/Climbables/BP_Ladder.BP_Ladder_C|GetTopZ _ladderparent))
          (Variables|Default|SetTypeSub (Variables|/Game/2DLadders/BluePrints/Climbables/BP_Ladder.BP_Ladder_C|GetSubType (Variables|Default|GetLadderParent)))
          (Components|Box|SetBoxExtent (Variables|Default|GetBox) (Math|Vector|MakeVector 32.0 15.0 (* (Math|Conversions|ToFloat(Integer) (Variables|/Game/2DLadders/BluePrints/Climbables/BP_Ladder.BP_Ladder_C|GetLength _ladderparent)) (/ (Variables|/Game/2DLadders/BluePrints/Climbables/BP_Ladder.BP_Ladder_C|GetSectionSize _ladderparent) 2.3))) true))))
    (:NewEnumerator3
      (Variables|Default|SetTop (Variables|/Game/2DLadders/BluePrints/Climbables/BP_ClimbWall.BP_ClimbWall_C|GetTopZ _wallparent))
      (Components|Box|SetBoxExtent (Variables|Default|GetBox) (Math|Vector|MakeVector 32.0 (* (Math|Conversions|ToFloat(Integer) (Variables|/Game/2DLadders/BluePrints/Climbables/BP_ClimbWall.BP_ClimbWall_C|GetWidth _wallparent)) (/ (Variables|/Game/2DLadders/BluePrints/Climbables/BP_ClimbWall.BP_ClimbWall_C|GetSectionSize _wallparent) 2.3)) (* (Math|Conversions|ToFloat(Integer) (Variables|/Game/2DLadders/BluePrints/Climbables/BP_ClimbWall.BP_ClimbWall_C|GetHight _wallparent)) (/ (Variables|/Game/2DLadders/BluePrints/Climbables/BP_ClimbWall.BP_ClimbWall_C|GetSectionSize _wallparent) 2.3))) true))))