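; Climbable wall for a 2.5D or Paper 2D platformer that can also shuttle back and forth.
; Construction script tiles a Width by Hight grid of meshes on Cube, adds an optional border and computes the travel endpoint.
; BeginPlay spawns and attaches a BP_ClimbVolume linked to the wall.
; While Moving, Tick drives Cube by interpolation or constant per-frame offsets, pausing for StopDelay before reversing at each end.
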(event Custom|Movement
  (params (Delta :type Float%20%28single-precision%29))
  ;[0.06818 0.1026 0.2396 1 30] Movement
  (if (Variables|Movement|GetMoving)
    (if (Variables|Movement|GetDelay)
      (Utilities|FlowControl|Delay (Variables|Movement|GetStopDelay))
      (Variables|Movement|SetDelay false)
      (else
        (CallFunction|MoveWall Delta)))))

(event EventBeginPlay
  (bind (_tiletransform _p2s_tiletransform _volumetransform _p2d_volumetransform) (Utilities|Transforms))
  (bind _self self)
  ;[1 0.3319 0.6767 1 30] SetClimbVolumes
  (switch Utilities|FlowControl|Switch|SwitchonEnum_PerspectiveWall (Variables|Main|GetPlatformerType)
    (:NewEnumerator0
      (bind _returnvalue (Game|SpawnActorfromClass "/Game/2DLadders/BluePrints/Climbables/BP_ClimbVolume.BP_ClimbVolume_C" _volumetransform "Undefined" 0 0 _self "NewEnumerator3" false 0))
      (bind _output_get (Variables|Default|SetVolume _returnvalue))
      (Transformation|AttachComponentToComponent (Variables|/Script/Engine.Actor|GetRootComponent _output_get) (Variables|Default|GetCube) "None" "KeepWorld" "KeepWorld" "KeepWorld" true))
    (:NewEnumerator1
      (bind _returnvalue_2 (Game|SpawnActorfromClass "/Game/2DLadders/BluePrints/Climbables/BP_ClimbVolume.BP_ClimbVolume_C" _p2d_volumetransform "Undefined" 0 0 _self "NewEnumerator3" false 0))
      (bind _output_get_2 (Variables|Default|SetVolume _returnvalue_2))
      (Transformation|AttachComponentToComponent (Variables|/Script/Engine.Actor|GetRootComponent _output_get_2) (Variables|Default|GetCube) "None" "KeepWorld" "KeepWorld" "KeepWorld" true))))

(event EventTick
  (params (DeltaSeconds :type Float%20%28single-precision%29))
  ;[0.06248 0.25 0.1323] Tick
  (CallFunction|Movement DeltaSeconds)
  (Variables|Default|SetCurrentPos (Transformation|GetWorldLocation (Variables|Default|GetCube))))

(fn ConstructionScript
  (bind _meshsections (Variables|Default|GetMeshSections))
  (bind _cube (Variables|Default|GetCube))
  (bind _output_get (Variables|Default|SetStartPos (Transformation|GetWorldLocation (Variables|Default|GetCube))))
  (switch Utilities|FlowControl|Switch|SwitchonEnum_MoveMethod (Variables|Movement|GetMoveMetod)
    (:NewEnumerator0
      (Variables|Default|SetMoveVectorts _output_get))
    (:NewEnumerator1
      _))
  (CallFunction|SetMovement)
  (Utilities|Array|Clear (Variables|Default|GetMeshSections))
  (CallFunction|Setup)
  (for _index (range 0 (- (Variables|Main|GetHight) 1))
    (for _index_2 (range 0 (- (Variables|Main|GetWidth) 1))
      (switch Utilities|FlowControl|Switch|SwitchonEnum_PerspectiveWall (Variables|Main|GetPlatformerType)
        (:NewEnumerator0
          (Utilities|Array|SetArrayElem _meshsections _index_2 "/Game/2DLadders/Props/SM_Metal_Ladder.SM_Metal_Ladder" true)
          (bind _returnvalue (AddComponent|AddStaticMeshComponent true (.TileTransform (Utilities|Transforms _index _index_2))))
          (Transformation|AttachComponentToComponent _returnvalue _cube "None" "KeepWorld" "KeepWorld" "KeepWorld" true))
        (:NewEnumerator1
          (Utilities|Array|SetArrayElem _meshsections 0 0 true)
          (bind _returnvalue_2 (AddComponent|AddStaticMeshComponent true (.P2S%20TileTransform (Utilities|Transforms _index _index_2))))
          (Transformation|AttachComponentToComponent _returnvalue_2 _cube "None" "KeepWorld" "KeepWorld" "KeepWorld" true)))))
  (Utilities|FlowControl|Sequence
    (:then_0
      (switch Utilities|FlowControl|Switch|SwitchonEnum_PerspectiveWall (Variables|Main|GetPlatformerType)
        (:NewEnumerator1
          (Transformation|SetWorldRotation (Variables|Default|GetCube) "0,90.000000, 0" false false))))
    (:then_1
      (if (Variables|Main|GetAddBorder)
        (CallFunction|Border (Transformation|GetWorldTransform (Variables|Default|GetCube)))))))

(fn Setup
  (bind _cube (Variables|Default|GetCube))
  (bind _sectionsize (Variables|Default|GetSectionSize))
  (bind _returnvalue (Transformation|GetWorldLocation _cube))
  (bind _z (Math|Vector|BreakVector _returnvalue))
  (Variables|Default|SetTopZ (+ _z _sectionsize))
  (Variables|Default|SetBotZ (+ (- _z (* (Math|Conversions|ToFloat(Integer) (Variables|Main|GetHight)) _sectionsize)) _sectionsize))
  (Variables|Main|SetHight (Math|Integer|Clamp(Integer) (Variables|Main|GetHight) 1 50))
  (Variables|Main|SetWidth (Math|Integer|Clamp(Integer) (Variables|Main|GetWidth) 1 50)))

(fn Border
  (params (RelativeTransform :type Transform))
  (bind _location (Math|Transform|BreakTransform RelativeTransform))
  (bind _location_2 (Math|Transform|BreakTransform RelativeTransform))
  (bind _location_3 (Math|Transform|BreakTransform RelativeTransform))
  (bind _location_4 (Math|Transform|BreakTransform RelativeTransform))
  (bind _width (Variables|Main|GetWidth))
  (bind _hight (Variables|Main|GetHight))
  (bind _sectionsize (Variables|Default|GetSectionSize))
  (bind _sectionsize_2 (Variables|Default|GetSectionSize))
  (bind _width_2 (Variables|Main|GetWidth))
  (bind _sectionsize_3 (Variables|Default|GetSectionSize))
  (bind _sectionsize_4 (Variables|Default|GetSectionSize))
  (bind _sectionsize_5 (Variables|Default|GetSectionSize))
  (bind _sectionsize_6 (Variables|Default|GetSectionSize))
  (bind _sectionsize_7 (Variables|Default|GetSectionSize))
  (bind _sectionsize_8 (Variables|Default|GetSectionSize))
  (bind _sectionsize_9 (Variables|Default|GetSectionSize))
  (bind (_x _y _z) (Math|Vector|BreakVector _location))
  (bind (_x_2 _y_2 _z_2) (Math|Vector|BreakVector _location_2))
  (bind _returnvalue (Math|Conversions|ToFloat(Integer) _width))
  (bind _returnvalue_2 (Math|Conversions|ToFloat(Integer) _hight))
  (bind (_x_3 _y_3 _z_3) (Math|Vector|BreakVector _location_2))
  (bind _returnvalue_3 (Math|Conversions|ToFloat(Integer) _width_2))
  (bind (_x_4 _y_4 _z_4) (Math|Vector|BreakVector _location_4))
  (bind (_x_5 _y_5 _z_5) (Math|Vector|BreakVector _location))
  (bind (_x_6 _y_6 _z_6) (Math|Vector|BreakVector _location_3))
  (bind (_x_7 _y_7 _z_7) (Math|Vector|BreakVector _location_3))
  (bind (_x_8 _y_8 _z_8) (Math|Vector|BreakVector _location_4))
  (bind _returnvalue_4 (Math|Vector|MakeVector 2.0 2.0 _returnvalue))
  (bind _returnvalue_5 (Math|Vector|MakeVector 2.0 2.0 _returnvalue_2))
  (bind _returnvalue_6 (Math|Vector|MakeVector 2.0 2.0 _returnvalue_3))
  (Utilities|FlowControl|Sequence
    (:then_0
      (switch Utilities|FlowControl|Switch|SwitchonEnum_PerspectiveWall (Variables|Main|GetPlatformerType)
        (:NewEnumerator0
          (bind _returnvalue_7 (AddComponent|AddStaticMeshComponent true (Math|Transform|MakeTransform (Math|Vector|MakeVector _x_2 (- _y_2 (- (* (Variables|Main|GetWidth) _sectionsize_6) (/ _sectionsize_6 2.0))) (+ _z_2 (/ (Variables|Default|GetSectionSize) 2.0))) "0.000000,0.000000,90.000000" _returnvalue_6)))
          (Transformation|AttachComponentToComponent _returnvalue_7 (Variables|Default|GetCube) "None" "KeepWorld" "KeepWorld" "KeepWorld" true))
        (:NewEnumerator1
          (bind _returnvalue_8 (AddComponent|AddStaticMeshComponent true (Math|Transform|MakeTransform (Math|Vector|MakeVector (+ _x_3 (- (* (Variables|Main|GetWidth) _sectionsize_3) (/ _sectionsize_3 2.0))) _y_3 (+ _z_3 (/ (Variables|Default|GetSectionSize) 2.0))) "0.000000,90.000000,90.000000" _returnvalue_6)))
          (Transformation|AttachComponentToComponent _returnvalue_8 (Variables|Default|GetCube) "None" "KeepWorld" "KeepWorld" "KeepWorld" true)
          (Collision|SetCollisionEnabled _returnvalue_8 "NoCollision"))))
    (:then_1
      (switch Utilities|FlowControl|Switch|SwitchonEnum_PerspectiveWall (Variables|Main|GetPlatformerType)
        (:NewEnumerator0
          (bind _returnvalue_9 (AddComponent|AddStaticMeshComponent true (Math|Transform|MakeTransform (Math|Vector|MakeVector _x_5 (- _y_5 (- (* (Variables|Main|GetWidth) _sectionsize_7) (/ _sectionsize_7 2.0))) (+ (- _z_5 (* (Variables|Main|GetHight) (Variables|Default|GetSectionSize))) (/ (Variables|Default|GetSectionSize) 2.0))) "0, 0,90.000000" _returnvalue_4)))
          (Transformation|AttachComponentToComponent _returnvalue_9 (Variables|Default|GetCube) "None" "KeepWorld" "KeepWorld" "KeepWorld" true))
        (:NewEnumerator1
          (bind _returnvalue_10 (AddComponent|AddStaticMeshComponent true (Math|Transform|MakeTransform (Math|Vector|MakeVector (+ _x (- (* (Variables|Main|GetWidth) _sectionsize_2) (/ _sectionsize_2 2.0))) _y (+ (- _z (* (Variables|Main|GetHight) (Variables|Default|GetSectionSize))) (/ (Variables|Default|GetSectionSize) 2.0))) "0,90.000000,90.000000" _returnvalue_4)))
          (Transformation|AttachComponentToComponent _returnvalue_10 (Variables|Default|GetCube) "None" "KeepWorld" "KeepWorld" "KeepWorld" true)
          (Collision|SetCollisionEnabled _returnvalue_10 "NoCollision"))))
    (:then_2
      (switch Utilities|FlowControl|Switch|SwitchonEnum_PerspectiveWall (Variables|Main|GetPlatformerType)
        (:NewEnumerator0
          (bind _returnvalue_11 (AddComponent|AddStaticMeshComponent true (Math|Transform|MakeTransform (Math|Vector|MakeVector _x_8 (+ _y_8 (/ (Variables|Default|GetSectionSize) 2.0)) (- _z_8 (- (* (Variables|Main|GetHight) _sectionsize_9) (/ _sectionsize_9 2.0)))) "0, 0, 0" (Math|Vector|MakeVector 2.0 2.0 (Math|Conversions|ToFloat(Integer) (Variables|Main|GetHight))))))
          (Transformation|AttachComponentToComponent _returnvalue_11 (Variables|Default|GetCube) "None" "KeepWorld" "KeepWorld" "KeepWorld" true))
        (:NewEnumerator1
          (bind _returnvalue_12 (AddComponent|AddStaticMeshComponent true (Math|Transform|MakeTransform (Math|Vector|MakeVector (- _x_4 (/ (Variables|Default|GetSectionSize) 2.0)) _y_4 (- _z_4 (- (* (Variables|Main|GetHight) _sectionsize_4) (/ _sectionsize_4 2.0)))) "0, 0, 0" (Math|Vector|MakeVector 2.0 2.0 (Math|Conversions|ToFloat(Integer) (Variables|Main|GetHight))))))
          (Transformation|AttachComponentToComponent _returnvalue_12 (Variables|Default|GetCube) "None" "KeepWorld" "KeepWorld" "KeepWorld" true)
          (Collision|SetCollisionEnabled _returnvalue_12 "NoCollision"))))
    (:then_3
      (switch Utilities|FlowControl|Switch|SwitchonEnum_PerspectiveWall (Variables|Main|GetPlatformerType)
        (:NewEnumerator0
          (bind _returnvalue_13 (AddComponent|AddStaticMeshComponent true (Math|Transform|MakeTransform (Math|Vector|MakeVector _x_7 (+ _y_7 (- (/ (Variables|Default|GetSectionSize) 2.0) (* (Variables|Main|GetWidth) (Variables|Default|GetSectionSize)))) (- _z_7 (- (* (Variables|Main|GetHight) _sectionsize_8) (/ _sectionsize_8 2.0)))) "0, 0, 0" _returnvalue_5)))
          (Transformation|AttachComponentToComponent _returnvalue_13 (Variables|Default|GetCube) "None" "KeepWorld" "KeepWorld" "KeepWorld" true))
        (:NewEnumerator1
          (bind _returnvalue_14 (AddComponent|AddStaticMeshComponent true (Math|Transform|MakeTransform (Math|Vector|MakeVector (+ _x_6 (+ (* (Variables|Main|GetWidth) (Variables|Default|GetSectionSize)) (- (/ _sectionsize 2.0) _sectionsize))) _y_6 (- _z_6 (- (* (Variables|Main|GetHight) _sectionsize_5) (/ _sectionsize_5 2.0)))) "0, 0, 0" _returnvalue_5)))
          (Transformation|AttachComponentToComponent _returnvalue_14 (Variables|Default|GetCube) "None" "KeepWorld" "KeepWorld" "KeepWorld" true)
          (Collision|SetCollisionEnabled _returnvalue_14 "NoCollision"))))))

(fn SetMovement
  (bind _startpos (Variables|Default|GetStartPos))
  (bind _startpos_2 (Variables|Default|GetStartPos))
  (bind _startpos_3 (Variables|Default|GetStartPos))
  (bind _startpos_4 (Variables|Default|GetStartPos))
  (bind _startpos_5 (Variables|Default|GetStartPos))
  (bind _startpos_6 (Variables|Default|GetStartPos))
  (bind _startpos_7 (Variables|Default|GetStartPos))
  (bind _startpos_8 (Variables|Default|GetStartPos))
  (bind (_x _y _z) (Math|Vector|BreakVector _startpos_6))
  (bind (_x_2 _y_2 _z_2) (Math|Vector|BreakVector _startpos_2))
  (bind (_x_3 _y_3 _z_3) (Math|Vector|BreakVector _startpos_3))
  (bind (_x_4 _y_4 _z_4) (Math|Vector|BreakVector _startpos_4))
  (bind (_x_5 _y_5 _z_5) (Math|Vector|BreakVector _startpos_5))
  (bind (_x_6 _y_6 _z_6) (Math|Vector|BreakVector _startpos_7))
  (bind (_x_7 _y_7 _z_7) (Math|Vector|BreakVector _startpos_8))
  (bind (_x_8 _y_8 _z_8) (Math|Vector|BreakVector _startpos))
  (Variables|Default|SetTopZ (+ (.Z (Math|Vector|BreakVector (Transformation|GetWorldLocation (Variables|Default|GetCube)))) (Variables|Default|GetSectionSize)))
  (switch Utilities|FlowControl|Switch|SwitchonEnum_PerspectiveWall (Variables|Main|GetPlatformerType)
    (:NewEnumerator0
      (switch Utilities|FlowControl|Switch|SwitchonEnum_direction (Variables|Movement|GetDirection)
        (:NewEnumerator0
          (bind _output_get (Variables|Default|SetEndPos (Math|Vector|MakeVector _x (- _y (* (Variables|Movement|GetTilesToMove) (Variables|Default|GetSectionSize))) _z)))
          (Variables|Default|SetTragetPos _output_get))
        (:NewEnumerator1
          (bind _output_get_2 (Variables|Default|SetEndPos (Math|Vector|MakeVector _x_7 (+ _y_7 (* (Variables|Movement|GetTilesToMove) (Variables|Default|GetSectionSize))) _z_7)))
          (Variables|Default|SetTragetPos _output_get_2))
        (:NewEnumerator2
          (bind _output_get_3 (Variables|Default|SetEndPos (Math|Vector|MakeVector _x_2 _y_2 (+ _z_2 (* (Variables|Movement|GetTilesToMove) (Variables|Default|GetSectionSize))))))
          (Variables|Default|SetTragetPos _output_get_3))
        (:NewEnumerator3
          (bind _output_get_4 (Variables|Default|SetEndPos (Math|Vector|MakeVector _x_8 _y_8 (- _z_8 (* (Variables|Movement|GetTilesToMove) (Variables|Default|GetSectionSize))))))
          (Variables|Default|SetTragetPos _output_get_4))))
    (:NewEnumerator1
      (switch Utilities|FlowControl|Switch|SwitchonEnum_direction (Variables|Movement|GetDirection)
        (:NewEnumerator0
          (bind _output_get_5 (Variables|Default|SetEndPos (Math|Vector|MakeVector (- _x_5 (* (Variables|Movement|GetTilesToMove) (Variables|Default|GetSectionSize))) _y_5 _z_5)))
          (Variables|Default|SetTragetPos _output_get_5))
        (:NewEnumerator1
          (bind _output_get_6 (Variables|Default|SetEndPos (Math|Vector|MakeVector (+ _x_6 (* (Variables|Movement|GetTilesToMove) (Variables|Default|GetSectionSize))) _y_6 _z_6)))
          (Variables|Default|SetTragetPos _output_get_6))
        (:NewEnumerator2
          (bind _output_get_7 (Variables|Default|SetEndPos (Math|Vector|MakeVector _x_3 _y_3 (+ _z_3 (* (Variables|Movement|GetTilesToMove) (Variables|Default|GetSectionSize))))))
          (Variables|Default|SetTragetPos _output_get_7))
        (:NewEnumerator3
          (bind _output_get_8 (Variables|Default|SetEndPos (Math|Vector|MakeVector _x_4 _y_4 (- _z_4 (* (Variables|Movement|GetTilesToMove) (Variables|Default|GetSectionSize))))))
          (Variables|Default|SetTragetPos _output_get_8))))))

(fn MoveWall
  (params (InputPin :type Float%20%28single-precision%29))
  (Variables|Default|SetTopZ (.Z (Math|Vector|BreakVector (Transformation|GetWorldLocation (Variables|Default|GetCube)))))
  (switch Utilities|FlowControl|Switch|SwitchonEnum_MoveMethod (Variables|Movement|GetMoveMetod)
    (:NewEnumerator0
      (Transformation|SetWorldLocation (Variables|Default|GetCube) (Variables|Default|GetMoveVectorts) false false)
      (switch Utilities|FlowControl|Switch|SwitchonEnum_BackForward (Variables|Movement|GetForwardBack)
        (:NewEnumerator0
          (Variables|Default|SetMoveVectorts (Math|Interpolation|VInterpTo (Variables|Default|GetMoveVectorts) (Variables|Default|GetEndPos) InputPin (Variables|Movement|GetMoveSpeed)))
          (if (Math|Vector|Equal(Vector) (Variables|Default|GetMoveVectorts) (Variables|Default|GetEndPos) 1e+01)
            (Variables|Movement|SetDelay true)
            (Variables|Movement|SetForwardBack "NewEnumerator1")))
        (:NewEnumerator1
          (Variables|Default|SetMoveVectorts (Math|Interpolation|VInterpTo (Variables|Default|GetMoveVectorts) (Variables|Default|GetStartPos) InputPin (Variables|Movement|GetMoveSpeed)))
          (if (Math|Vector|Equal(Vector) (Variables|Default|GetMoveVectorts) (Variables|Default|GetStartPos) 1e+01)
            (Variables|Movement|SetDelay true)
            (Variables|Movement|SetForwardBack "NewEnumerator0")))))
    (:NewEnumerator1
      (Transformation|AddWorldOffset (Variables|Default|GetCube) (Variables|Default|GetMoveVectorts) false false)
      (switch Utilities|FlowControl|Switch|SwitchonEnum_direction (Variables|Movement|GetDirection)
        (:NewEnumerator0
          (Variables|Default|SetMoveVectorts (Math|Vector|MakeVector 0.0 (* (Variables|Movement|GetMoveSpeed) -1.0) 0.0))
          (if (Math|Vector|Equal(Vector) (Variables|Default|GetCurrentPos) (Variables|Default|GetTragetPos) 1e+01)
            (Variables|Movement|SetDelay true)
            (Variables|Movement|SetDirection "NewEnumerator1")
            (switch Utilities|FlowControl|Switch|SwitchonEnum_BackForward (Variables|Movement|GetForwardBack) :!label _label
              (:NewEnumerator0
                (Variables|Default|SetTragetPos (Variables|Default|GetStartPos))
                (Variables|Movement|SetForwardBack "NewEnumerator1"))
              (:NewEnumerator1
                (Variables|Default|SetTragetPos (Variables|Default|GetEndPos))
                (Variables|Movement|SetForwardBack "NewEnumerator0")))))
        (:NewEnumerator1
          (Variables|Default|SetMoveVectorts (Math|Vector|MakeVector 0.0 (Variables|Movement|GetMoveSpeed) 0.0))
          (if (Math|Vector|Equal(Vector) (Variables|Default|GetCurrentPos) (Variables|Default|GetTragetPos) 1e+01)
            (Variables|Movement|SetDelay true)
            (Variables|Movement|SetDirection "NewEnumerator0")
            (goto _label)))
        (:NewEnumerator2
          (Variables|Default|SetMoveVectorts (Math|Vector|MakeVector 0.0 0.0 (Variables|Movement|GetMoveSpeed)))
          (if (Math|Vector|Equal(Vector) (Variables|Default|GetCurrentPos) (Variables|Default|GetTragetPos) 1e+01)
            (Variables|Movement|SetDelay true)
            (Variables|Movement|SetDirection "NewEnumerator3")
            (goto _label)))
        (:NewEnumerator3
          (Variables|Default|SetMoveVectorts (Math|Vector|MakeVector 0.0 0.0 (* (Variables|Movement|GetMoveSpeed) -1.0)))
          (if (Math|Vector|Equal(Vector) (Variables|Default|GetCurrentPos) (Variables|Default|GetTragetPos) 1e+01)
            (Variables|Movement|SetDelay true)
            (Variables|Movement|SetDirection "NewEnumerator2")
            (goto _label)))))))