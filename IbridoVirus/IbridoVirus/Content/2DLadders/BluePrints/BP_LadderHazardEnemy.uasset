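; A hazard enemy for 2D ladders that patrols vertically along its attached ladder.
; The construction script attaches it to LadderAttached and places its Sphere on a clamped StartTile, measured downward from the ladder's Cube by section size.
; Tick offsets the Sphere without sweep and flips Direction at the ladder's top and bottom Z limits, using separate up and down speeds.
; Overlap with BP_LadderCharacter only prints a hurt message.
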(event OnComponentBeginOverlap(Sphere)
  (params (OverlappedComponent :type Primitive%20Component%20Object%20Reference) (OtherActor :type Actor%20Object%20Reference) (OtherComp :type Primitive%20Component%20Object%20Reference) (OtherBodyIndex :type Integer) (bFromSweep :type Boolean) (SweepResult :type Hit%20Result%20Structure%20%28by%20ref%29))
  (Utilities|Casting|CastToBP_LadderCharacter OtherActor)
  (Development|PrintString "owch!"))

(event EventTick
  (params (DeltaSeconds :type Float%20%28single-precision%29))
  (bind _sphere (Variables|Default|GetSphere))
  (bind _ladderattached (Variables|Default|GetLadderAttached))
  (bind _returnvalue (Transformation|GetWorldLocation _sphere))
  (bind _z (Math|Vector|BreakVector _returnvalue))
  (Transformation|AddWorldOffset _sphere (Math|Vector|MakeVector 0.0 0.0 (Variables|Default|GetZspeed)) false false)
  (switch Utilities|FlowControl|Switch|SwitchonEnum_direction (Variables|Default|GetDirection)
    (:NewEnumerator2
      (Variables|Default|SetZspeed (Variables|Default|GetUpSpeed))
      (if (>= _z (Variables|/Game/2DLadders/BluePrints/Climbables/BP_Ladder.BP_Ladder_C|GetTopZ _ladderattached))
        (Variables|Default|SetDirection "NewEnumerator3")))
    (:NewEnumerator3
      (Variables|Default|SetZspeed (Variables|Default|GetDownSpeed))
      (if (<= _z (Variables|/Game/2DLadders/BluePrints/Climbables/BP_Ladder.BP_Ladder_C|GetBotZ _ladderattached))
        (Variables|Default|SetDirection "NewEnumerator2")))))

(fn ConstructionScript
  (bind _ladderattached (Variables|Default|GetLadderAttached))
  (bind _cube (Variables|/Game/2DLadders/BluePrints/Climbables/BP_Ladder.BP_Ladder_C|GetCube _ladderattached))
  (bind _sectionsize (Variables|/Game/2DLadders/BluePrints/Climbables/BP_Ladder.BP_Ladder_C|GetSectionSize _ladderattached))
  (bind _returnvalue (Transformation|GetWorldLocation _cube))
  (bind (_x _y _z) (Math|Vector|BreakVector _returnvalue))
  (Transformation|AttachActorToActor _ladderattached "None" "SnapToTarget" "KeepWorld" "KeepWorld" true)
  (Variables|Default|SetstartTile (Math|Integer|Clamp(Integer) (Variables|Default|GetstartTile) 1 (Variables|/Game/2DLadders/BluePrints/Climbables/BP_Ladder.BP_Ladder_C|GetLength _ladderattached)))
  (Transformation|SetWorldLocation (Variables|Default|GetSphere) (Math|Vector|MakeVector _x _y (+ (- _z (* (Variables|Default|GetstartTile) _sectionsize)) _sectionsize)) false false))